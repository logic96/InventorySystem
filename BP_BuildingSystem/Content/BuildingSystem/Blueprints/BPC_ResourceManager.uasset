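; Actor component for the building system that tracks the player's resource amounts and which resource is currently selected.
; Initialization caches the character, has the main widget generate per-resource widgets, then fills and highlights them.
; Adds and removals clamp amounts in a class-keyed map and refresh the matching widget, notifying the building manager for the selected resource in one character state.
; Cycling selection wraps around, updates the UI and notifies the building manager.
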(event `OnResourceSwitch`
  (`/Game/BuildingSystem/Blueprints/BPC_BuildingManager.OnResourceChanged` (`/Game/ThirdPersonBP/Blueprints/ThirdPersonCharacter.BPC_BuildingManager` (`self.CharacterRef`))))

(event `InitializeManager`
  (params (Player :type "/Game/ThirdPersonBP/Blueprints/ThirdPersonCharacter Object Reference"))
  (`/Engine/EditorBlueprintResources/StandardMacros.IsValid` Player
    (:`Is Valid`
      (set `self.CharacterRef` Player)
      (set `self.Initialized?` true)
      (bind _createdwidgets (`/Game/BuildingSystem/Widgets/W_Main.GenerateResourceWidgets` (`/Game/ThirdPersonBP/Blueprints/ThirdPersonCharacter.MainWidgetRef` (`self.CharacterRef`)) self))
      (set `self.ResourceWidgets` _createdwidgets)
      (bind _keys (`BlueprintMapLibrary.Map_Keys` (`self.Resources`)))
      (for _array_element _keys
        (`self.UpdateResourceDisplay` _array_element))
      (`self.SelectCurrentResource`))))

(fn `AddResource`
  (params (Resource :type "/Game/BuildingSystem/Blueprints/Resources/BP_Master_Resources Class Reference") (Amount :type Integer))
  (locals (LocalResource :type "/Game/BuildingSystem/Blueprints/Resources/BP_Master_Resources Class Reference") (LocalAmount :type Integer))
  (bind (_value _returnvalue) (`BlueprintMapLibrary.Map_Find` (`self.Resources`) (`local.LocalResource`)))
  (set `local.LocalResource` Resource)
  (set `local.LocalAmount` Amount)
  (if (and (`KismetSystemLibrary.IsValidClass` Resource) (> Amount 0))
    (if _returnvalue
      (`BlueprintMapLibrary.Map_Add` (`self.Resources`) (`local.LocalResource`) (`KismetMathLibrary.Clamp` (+ _value (`local.LocalAmount`)) 0 999))
      (else
        (`BlueprintMapLibrary.Map_Add` (`self.Resources`) (`local.LocalResource`) (`KismetMathLibrary.Clamp` (`local.LocalAmount`) 0 999))))
    (`self.UpdateResourceDisplay` (`local.LocalResource`))
    (return)
    (else
      (return))))

(fn `GetCurrentlySelectedWidget`
  (returns (Widget :type "/Game/BuildingSystem/Widgets/W_Resource Object Reference"))
  (return (`.Widget` (`self.GetWidgetForResource` (`self.GetSelectedResource`)))))

(fn `GetResourceAmount`
  (params (Resource :type "/Game/BuildingSystem/Blueprints/Resources/BP_Master_Resources Class Reference"))
  (returns (Amount :type Integer))
  (bind (_value _returnvalue) (`BlueprintMapLibrary.Map_Find` (`self.Resources`) Resource))
  (if _returnvalue
    (return _value)
    (else
      (return -1))))

(fn `GetSelectedIndex`
  (returns (SelectedResourceIndex :type Integer))
  (return (`self.SelectedResourceIndex`)))

(fn `GetSelectedResource`
  (returns (Output :type "/Game/BuildingSystem/Blueprints/Resources/BP_Master_Resources Class Reference"))
  (bind _keys (`BlueprintMapLibrary.Map_Keys` (`self.Resources`)))
  (return (`|GetArrayItem` _keys (`self.SelectedResourceIndex`))))

(fn `GetWidgetForResource`
  (params (Resource :type "/Game/BuildingSystem/Blueprints/Resources/BP_Master_Resources Class Reference"))
  (returns (`Sucess?` :type Boolean) (Widget :type "/Game/BuildingSystem/Widgets/W_Resource Object Reference"))
  (for _array_element (`self.ResourceWidgets`)
    (if (== Resource (`/Game/BuildingSystem/Widgets/W_Resource.Resource` _array_element))
      (return true _array_element)))
  (return false null))

(fn `RemoveResource`
  (params (Resource :type "/Game/BuildingSystem/Blueprints/Resources/BP_Master_Resources Class Reference") (Amount :type Integer))
  (locals (LocalResource :type "/Game/BuildingSystem/Blueprints/Resources/BP_Master_Resources Class Reference") (LocalAmount :type Integer))
  (bind (_value _returnvalue) (`BlueprintMapLibrary.Map_Find` (`self.Resources`) (`local.LocalResource`)))
  (set `local.LocalResource` Resource)
  (set `local.LocalAmount` Amount)
  (if (and (`KismetSystemLibrary.IsValidClass` Resource) (> Amount 0))
    (if _returnvalue
      (`BlueprintMapLibrary.Map_Add` (`self.Resources`) (`local.LocalResource`) (`KismetMathLibrary.Clamp` (- _value (`local.LocalAmount`)) 0 999))
      (`self.UpdateResourceDisplay` (`local.LocalResource`))
      (return)
      (else
        (return)))
    (else
      (return))))

(fn `SelectCurrentResource`
  (`/Game/BuildingSystem/Widgets/W_Resource.SelectResource` (`self.GetCurrentlySelectedWidget`) true false)
  (return))

(fn `SelectNextResource`
  (bind _selectedresourceindex (`self.SelectedResourceIndex`))
  ;[1 1 1] 当前有选取态取消
  (`/Game/BuildingSystem/Widgets/W_Resource.SelectResource` (`self.GetCurrentlySelectedWidget`) false false)
  (bind _keys (`BlueprintMapLibrary.Map_Keys` (`self.Resources`)))
  (set `self.SelectedResourceIndex` (`KismetMathLibrary.SelectInt` (+ _selectedresourceindex 1) 0 (< _selectedresourceindex (`KismetArrayLibrary.Array_LastIndex` _keys))))
  (`self.SelectCurrentResource`)
  (`/Game/BuildingSystem/Widgets/W_Main.UpdateCurrentResources` (`/Game/ThirdPersonBP/Blueprints/ThirdPersonCharacter.MainWidgetRef` (`self.CharacterRef`)) self)
  ;[1 1 1] 触发Switch事件
  (`self.OnResourceSwitch`))

(fn `UpdateResourceDisplay`
  (params (Resource :type "/Game/BuildingSystem/Blueprints/Resources/BP_Master_Resources Class Reference"))
  (bind (_sucess_ _widget) (`self.GetWidgetForResource` Resource))
  (if (`self.Initialized?`)
    (if _sucess_
      (`TextBlock.SetText` (`/Game/BuildingSystem/Widgets/W_Resource.AmountText` _widget) (`KismetTextLibrary.Conv_IntToText` (`self.GetResourceAmount` Resource)))
      (if (and (== (`self.GetSelectedResource`) Resource) (`|EnumEquality` (`/Game/ThirdPersonBP/Blueprints/ThirdPersonCharacter.State` (`self.CharacterRef`)) "NewEnumerator1"))
        (`/Game/BuildingSystem/Widgets/W_Main.UpdateCurrentResources` (`/Game/ThirdPersonBP/Blueprints/ThirdPersonCharacter.MainWidgetRef` (`self.CharacterRef`)) self)
        (`/Game/BuildingSystem/Blueprints/BPC_BuildingManager.OnResourceValueModified` (`/Game/ThirdPersonBP/Blueprints/ThirdPersonCharacter.BPC_BuildingManager` (`self.CharacterRef`)) Resource)))))
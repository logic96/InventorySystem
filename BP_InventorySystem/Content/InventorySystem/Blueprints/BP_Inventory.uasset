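; Slot-based inventory actor that stores item class and amount pairs and creates the main widget that displays them.
; AddItem recursively spreads amounts over stacks and empty slots up to MaxStackSize, with a wrapper that queues pickup messages on the widget.
; Remove, swap, split and merge operations refresh affected slot widgets through OnSlotChanged.
; Using an item spawns its actor, calls OnUse and removes one if a consumable succeeds.
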(event `self.ReceiveBeginPlay`
  (`KismetArrayLibrary.Array_Resize` (`self.Slots`) (`self.AmountOfSlots`))
  ;[1 1 1] 正常来讲这部分应该放在Character中
  (bind _returnvalue (`|CreateWidget` "/Game/InventorySystem/Widget/W_MainWidget.W_MainWidget_C" null self (`self.SlotsPerRow`) 0.5))
  (bind _output_get (set `self.MainWidgetRef` _returnvalue))
  (set `self.InventoryWidgetRef` (`/Game/InventorySystem/Widget/W_MainWidget.InventoryWidget` _output_get))
  (`UserWidget.AddToViewport` (`self.MainWidgetRef`) 0))

(event `OnSlotChanged`
  (params (Index :type Integer))
  ;[1 1 1] 只要Slot内元素发生改变就需要调用该事件函数
  (`self.UpdateSlotAtIndex` Index))

(fn `AddItem`
  (params (ItemToAdd :type "/Game/InventorySystem/Blueprints/ItemClasses/BP_MasterItem Class Reference") (Amount :type Integer))
  (returns (`Sucess?` :type Boolean) (Rest :type Integer))
  (locals (LocalAmount :type Integer) (LocalItemClass :type "/Game/InventorySystem/Blueprints/ItemClasses/BP_MasterItem Class Reference") (LocalIndex :type Integer :default 0))
  ;[1 1 1] 首先看是否能够堆积，对于魔女之泉，默认都可以堆积
  (set `local.LocalAmount` Amount)
  (set `local.LocalItemClass` ItemToAdd)
  (if (`.CanbeStacked?_18_D6105F594C4B0FE84DD61F97824154B7` (break `/Game/InventorySystem/Blueprints/S_ItemInfo` (defaults `/Game/InventorySystem/Blueprints/BP_Inventory` ItemToAdd)))
    ;[1 1 1] 能堆积的话，先找freestack
    (bind (_sucess_ _index) (`self.SearchFreeStack` (`local.LocalItemClass`)))
    (if _sucess_
      (bind _output_get (set `local.LocalIndex` _index))
      (bind _returnvalue (+ (`.Amount_5_F101883A4AEB044BD29A47BA0494C110` (break `/Game/InventorySystem/Blueprints/S_InventorySlot` (`|GetArrayItem` (`self.Slots`) _output_get))) (`local.LocalAmount`)))
      (if (>= (`self.MaxStackSize`) _returnvalue)
        ;[1 1 1] 魔女之泉执行这里，堆积到已有栏
        (`KismetArrayLibrary.Array_Set` (`self.Slots`) (`local.LocalIndex`) (make `/Game/InventorySystem/Blueprints/S_InventorySlot` (`local.LocalItemClass`) _returnvalue))
        (`self.OnSlotChanged` (`local.LocalIndex`))
        (return true 0)
        (else
          (bind _output_get_2 (set `local.LocalAmount` (- _returnvalue (`self.MaxStackSize`)))) ; 需要在setArrayElemt前重新设置LocalAmount
          (`KismetArrayLibrary.Array_Set` (`self.Slots`) (`local.LocalIndex`) (make `/Game/InventorySystem/Blueprints/S_InventorySlot` (`local.LocalItemClass`) (`self.MaxStackSize`)))
          (`self.OnSlotChanged` (`local.LocalIndex`))
          (bind (_sucess__2 _rest) (`self.AddItem` (`local.LocalItemClass`) _output_get_2))
          (return _sucess__2 _rest)))
      (else
        ;[1 1 1] 找不到freestack,才找空槽
        (bind (_sucess__3 _index_2) (`self.SearchEmptySlot`))
        (if _sucess__3
          (set `local.LocalIndex` _index_2)
          ;[1 1 1] 找到的话还要看一个格能不能放得下
          (if (>= (`self.MaxStackSize`) (`local.LocalAmount`))
            ;[1 1 1] 魔女之泉执行这里(当前列表没有，进行堆积)
            (`KismetArrayLibrary.Array_Set` (`self.Slots`) (`local.LocalIndex`) (make `/Game/InventorySystem/Blueprints/S_InventorySlot` (`local.LocalItemClass`) (`local.LocalAmount`)))
            ;[1 1 1] slot变化事件调用
            (`self.OnSlotChanged` (`local.LocalIndex`))
            (return true 0)
            (else
              (`KismetArrayLibrary.Array_Set` (`self.Slots`) (`local.LocalIndex`) (make `/Game/InventorySystem/Blueprints/S_InventorySlot` (`local.LocalItemClass`) (`self.MaxStackSize`)))
              ;[1 1 1] slot变化事件调用
              (`self.OnSlotChanged` (`local.LocalIndex`))
              (bind (_sucess__4 _rest_2) (`self.AddItem` (`local.LocalItemClass`) (- (`local.LocalAmount`) (`self.MaxStackSize`))))
              (return _sucess__4 _rest_2)))
          (else
            ;[1 1 1] 找不到空槽的话，就返回false
            (return false (`local.LocalAmount`))))))
    (else
      ;[1 1 1] 不能堆积的话，就找空槽
      (bind (_sucess__5 _index_3) (`self.SearchEmptySlot`))
      (if _sucess__5
        ;[1 1 1] 找到的话，就在当前格放一个
        (bind _output_get_3 (set `local.LocalIndex` _index_3))
        (`KismetArrayLibrary.Array_Set` (`self.Slots`) _output_get_3 (make `/Game/InventorySystem/Blueprints/S_InventorySlot` (`local.LocalItemClass`) 1))
        ;[1 1 1] slot变化事件调用
        (`self.OnSlotChanged` (`local.LocalIndex`))
        (if (> (`local.LocalAmount`) 1)
          ;[1 1 1] 递归添加
          (bind (_sucess__6 _rest_3) (`self.AddItem` (`local.LocalItemClass`) (- (`local.LocalAmount`) 1)))
          (return _sucess__6 _rest_3)
          (else
            (return true 0) ; 递归正常结束
          ))
        (else
          ;[1 1 1] 找不到空槽的话，就返回false
          (return false (`local.LocalAmount`)))))))

(fn `AddItemAndShowMessage`
  (params (ItemClass :type "/Game/InventorySystem/Blueprints/ItemClasses/BP_MasterItem Class Reference") (Amount :type Integer))
  (returns (`Sucess?` :type Boolean) (Rest :type Integer))
  (bind (_sucess_ _rest) (`self.AddItem` ItemClass Amount))
  (if _sucess_
    ;[1 1 1] 将添加成功的记录在案
    (`/Game/InventorySystem/Widget/W_MainWidget.AddItemToPickUpsQueue` (`self.MainWidgetRef`) ItemClass (- Amount _rest))
    (return true _rest)
    (else
      (return false _rest))))

(fn `AddToIndex`
  (params (FromIndex :type Integer) (ToIndex :type Integer))
  (returns (`Sucess?` :type Boolean))
  (locals (From :type Integer) (To :type Integer) (LocalClass :type "/Game/InventorySystem/Blueprints/ItemClasses/BP_MasterItem Class Reference"))
  (bind _itemclass (break `/Game/InventorySystem/Blueprints/S_InventorySlot` (`|GetArrayItem` (`self.Slots`) (`local.From`))))
  (bind (_itemclass_2 _amount) (break `/Game/InventorySystem/Blueprints/S_InventorySlot` (`|GetArrayItem` (`self.Slots`) (`local.To`))))
  (set `local.From` FromIndex)
  (set `local.To` ToIndex)
  (if (and (== _itemclass _itemclass_2) (< _amount (`self.MaxStackSize`)) (`.CanbeStacked?_18_D6105F594C4B0FE84DD61F97824154B7` (break `/Game/InventorySystem/Blueprints/S_ItemInfo` (`.ItemInfo` (`self.GetItemInfoAtIndex` (`local.From`))))))
    (set `local.LocalClass` _itemclass)
    (if (>= (- (`self.MaxStackSize`) (`self.GetAmountAtIndex` (`local.To`))) (`self.GetAmountAtIndex` (`local.From`)))
      ;[1 1 1] 先改To再改from
      (`KismetArrayLibrary.Array_Set` (`self.Slots`) (`local.To`) (make `/Game/InventorySystem/Blueprints/S_InventorySlot` (`local.LocalClass`) (+ (`self.GetAmountAtIndex` (`local.To`)) (`self.GetAmountAtIndex` (`local.From`)))))
      (`KismetArrayLibrary.Array_Set` (`self.Slots`) (`local.From`) (make `/Game/InventorySystem/Blueprints/S_InventorySlot` null))
      (`self.OnSlotChanged` (`local.From`))
      (`self.OnSlotChanged` (`local.To`))
      (return true)
      (else
        ;[1 1 1] 注意先改From，再改To,
        (`KismetArrayLibrary.Array_Set` (`self.Slots`) (`local.From`) (make `/Game/InventorySystem/Blueprints/S_InventorySlot` (`local.LocalClass`) (- (+ (`self.GetAmountAtIndex` (`local.To`)) (`self.GetAmountAtIndex` (`local.From`))) (`self.MaxStackSize`))))
        (`KismetArrayLibrary.Array_Set` (`self.Slots`) (`local.To`) (make `/Game/InventorySystem/Blueprints/S_InventorySlot` (`local.LocalClass`) (`self.MaxStackSize`)))
        (`self.OnSlotChanged` (`local.From`))
        (`self.OnSlotChanged` (`local.To`))
        (return true)))
    (else
      (return false))))

(fn `GetAmountAtIndex`
  (params (Index :type Integer))
  (returns (Amount :type Integer))
  (return (`.Amount_5_F101883A4AEB044BD29A47BA0494C110` (break `/Game/InventorySystem/Blueprints/S_InventorySlot` (`|GetArrayItem` (`self.Slots`) Index)))))

(fn `GetItemInfoAtIndex`
  (params (Index :type Integer))
  (returns (`IsEmpty?` :type Boolean) (ItemInfo :type "/Game/InventorySystem/Blueprints/S_ItemInfo Structure") (Amount :type Integer))
  (bind (_itemclass _amount) (break `/Game/InventorySystem/Blueprints/S_InventorySlot` (`|GetArrayItem` (`self.Slots`) Index)))
  (return (not (`KismetSystemLibrary.IsValidClass` _itemclass)) (defaults `/Game/InventorySystem/Blueprints/BP_Inventory` _itemclass) _amount))

(fn `HideInventory`
  (`Widget.SetVisibility` (`self.InventoryWidgetRef`) "Hidden")
  (set `self.IsVisible?` false)
  (`Widget.SetIsEnabled` (`self.InventoryWidgetRef`) false)
  (return))

(fn `IsSlotEmpty`
  (params (Index :type Integer))
  (returns (`Empty?` :type Boolean))
  (return (not (`KismetSystemLibrary.IsValidClass` (`.ItemClass_2_9032458A4767DB0AD509078831766904` (break `/Game/InventorySystem/Blueprints/S_InventorySlot` (`|GetArrayItem` (`self.Slots`) Index)))))))

(fn `RemoveItemAtIndex`
  (params (Index :type Integer) (Amount :type Integer))
  (returns (`Sucess?` :type Boolean))
  (locals (LocalIndex :type Integer) (LocalAmount :type Integer))
  (bind _slots (`self.Slots`))
  (bind _localindex (`local.LocalIndex`))
  (bind (_output_itemclass _output_amount) (break `/Game/InventorySystem/Blueprints/S_InventorySlot` (`|GetArrayItem` _slots _localindex)))
  (bind _output_get (set `local.LocalIndex` Index))
  (bind _output_get_2 (set `local.LocalAmount` Amount))
  (if (`self.IsSlotEmpty` _output_get)
    (return false) ; slot为空，移除失败
    (elif (> _output_get_2 0)
      (if (>= (`local.LocalAmount`) (`self.GetAmountAtIndex` (`local.LocalIndex`)))
        ;[1 1 1] 要移除的数目大于等于已有数目，则清空该slot
        (`KismetArrayLibrary.Array_Set` (`self.Slots`) (`local.LocalIndex`) (make `/Game/InventorySystem/Blueprints/S_InventorySlot` null))
        ;[1 1 1] 只要slot元素发生变化，就调用
        (`self.OnSlotChanged` (`local.LocalIndex`))
        (return true)
        (else
          ;[1 1 1] 正常的调用走这
          (`KismetArrayLibrary.Array_Set` _slots _localindex (make `/Game/InventorySystem/Blueprints/S_InventorySlot` _output_itemclass (- _output_amount (`local.LocalAmount`))))
          ;[1 1 1] 只要slot元素发生变化，就调用
          (`self.OnSlotChanged` (`local.LocalIndex`))
          (return true)))
      (else
        (return false) ; 移除的数目为空，失败
      ))))

(fn `SearchEmptySlot`
  (returns (`Sucess?` :type Boolean) (Index :type Integer))
  (locals (LocalIndex :type Integer) (Localbool :type Boolean :default false))
  (for (_ _array_index) (`self.Slots`)
    (if (`self.IsSlotEmpty` _array_index)
      (return true _array_index)))
  (return false 0) ; 一圈没找到，则返回false
)

(fn `SearchFreeStack`
  (params (ItemClass :type "/Game/InventorySystem/Blueprints/ItemClasses/BP_MasterItem Class Reference"))
  (returns (`Sucess?` :type Boolean) (Index :type Integer))
  (locals (NewLocalVar_0 :type Integer))
  (for (_array_element _array_index) (`self.Slots`)
    (if (`self.IsSlotEmpty` _array_index)
      (return false 0)
      (else
        (bind (_itemclass _amount) (break `/Game/InventorySystem/Blueprints/S_InventorySlot` _array_element))
        (if (and (== _itemclass ItemClass) (< _amount (`self.MaxStackSize`)))
          (return true _array_index) ; 只有当前槽中不为空且未满时返回true
          (else
            (return false 0))))))
  (return false 0))

(fn `ShowInventory`
  (`Widget.SetVisibility` (`self.InventoryWidgetRef`) "Visible")
  (set `self.IsVisible?` true)
  (`Widget.SetIsEnabled` (`self.InventoryWidgetRef`) true)
  (return))

(fn `SplitStack`
  (params (StackIndex :type Integer) (Amount :type Integer))
  (returns (`Sucess?` :type Boolean))
  (locals (LocalStackIndex :type Integer) (LocalAmount :type Integer))
  (bind _localstackindex (`local.LocalStackIndex`))
  (bind _slots (`self.Slots`))
  (bind (_isempty_ _iteminfo _amount) (`self.GetItemInfoAtIndex` (`local.LocalStackIndex`)))
  (bind (_output_itemclass _output_amount) (break `/Game/InventorySystem/Blueprints/S_InventorySlot` (`|GetArrayItem` _slots _localstackindex)))
  (set `local.LocalStackIndex` StackIndex)
  (set `local.LocalAmount` Amount)
  (if (`self.IsSlotEmpty` StackIndex)
    (return false) ; 空栏无法分
    (elif (and (`.CanbeStacked?_18_D6105F594C4B0FE84DD61F97824154B7` (break `/Game/InventorySystem/Blueprints/S_ItemInfo` _iteminfo)) (> _amount (`local.LocalAmount`)))
      (bind (_sucess_ _index) (`self.SearchEmptySlot`))
      (if _sucess_
        (`KismetArrayLibrary.Array_Set` _slots _localstackindex (make `/Game/InventorySystem/Blueprints/S_InventorySlot` _output_itemclass (- _output_amount (`local.LocalAmount`))))
        (`KismetArrayLibrary.Array_Set` (`self.Slots`) _index (make `/Game/InventorySystem/Blueprints/S_InventorySlot` _output_itemclass (`local.LocalAmount`)))
        (`self.OnSlotChanged` _index)
        (`self.OnSlotChanged` (`local.LocalStackIndex`))
        (return true)
        (else
          (return false) ; 空栏无法分
        ))
      (else
        (return false) ; 空栏无法分
      ))))

(fn `SwapSlots`
  (params (Index1 :type Integer) (Index2 :type Integer))
  (returns (`Sucess?` :type Boolean))
  (if (or (> Index1 (`KismetArrayLibrary.Array_LastIndex` (`self.Slots`))) (> Index2 (`KismetArrayLibrary.Array_LastIndex` (`self.Slots`))))
    (return false)
    (else
      (`KismetArrayLibrary.Array_Swap` (`self.Slots`) Index1 Index2) ; 调用前检查数组越界
      ;[1 1 1] Swap也需要调用OnChanged
      (`self.OnSlotChanged` Index1)
      (`self.OnSlotChanged` Index2)
      (return true))))

(fn `UpdateSlotAtIndex`
  (params (Index :type Integer))
  (`/Game/InventorySystem/Widget/W_InventorySlot.UpdateSlot` (`|GetArrayItem` (`/Game/InventorySystem/Widget/W_Inventory.AllItem_SlotWidgets` (`self.InventoryWidgetRef`)) Index)))

(fn `UseItemAtIndex`
  (params (Index :type Integer))
  (locals (localIndex :type Integer))
  (bind _itemclass (break `/Game/InventorySystem/Blueprints/S_InventorySlot` (`|GetArrayItem` (`self.Slots`) Index)))
  (set `local.localIndex` Index)
  (if (`KismetSystemLibrary.IsValidClass` _itemclass)
    (bind _returnvalue (`|SpawnActorFromClass` _itemclass (`KismetMathLibrary.MakeTransform` (0.0 0.0 0.0)) "AlwaysSpawn" "OverrideRootScale" null self null))
    (bind _sucess_ (`/Game/InventorySystem/Blueprints/ItemClasses/BP_MasterItem.OnUse` _returnvalue)) ; 会调用各个物品的OnUse
    (if _sucess_
      (switch `/Game/InventorySystem/Blueprints/E_ItemCategory` (`.Category_21_387033E74DD616C3E78DFCA589DB38B3` (break `/Game/InventorySystem/Blueprints/S_ItemInfo` (`.ItemInfo` (`self.GetItemInfoAtIndex` (`local.localIndex`)))))
        (:`NewEnumerator0`
          ;[1 1 1] 使用成功时，根据道具类型决定是否remove
          (`self.RemoveItemAtIndex` (`local.localIndex`) 1)
          (return))
        (:`NewEnumerator1`
          _)
        (:`NewEnumerator2`
          _)
        (:`NewEnumerator3`
          _))
      (return)
      (else
        (return)))
    (else
      (return))))

(fn `UserConstructionScript`)
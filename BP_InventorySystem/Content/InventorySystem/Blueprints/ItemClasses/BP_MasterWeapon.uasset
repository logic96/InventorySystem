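; Base weapon item for the inventory system that equips and unequips itself on the owning TopDownCharacter.
; OnUse casts the inventory's character reference, adds a skeletal mesh component to itself at runtime using WeaponMesh, then passes itself to EquipWeapon.
; NotUse calls UnEquipWeapon on the character without removing the added component.
; Both functions return the character's result, or false if the cast fails.
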(fn `NotUse`
  (returns (`Sucess?` :type Boolean))
  (bind _astop_down_character (cast `/Game/TopDownBP/Blueprints/TopDownCharacter` (`/Game/InventorySystem/Blueprints/BP_Inventory.CharacterRef` (`self.InventoryRef`)))
    (:`then`
      (bind _sucess (`/Game/TopDownBP/Blueprints/TopDownCharacter.UnEquipWeapon` _astop_down_character))
      (return _sucess))
    (:`CastFailed`
      (return false))))

(fn `OnUse`
  (returns (`Sucess?` :type Boolean))
  (bind _astop_down_character (cast `/Game/TopDownBP/Blueprints/TopDownCharacter` (`/Game/InventorySystem/Blueprints/BP_Inventory.CharacterRef` (`self.InventoryRef`)))
    (:`then`
      ;[1 1 1] 动态的添加Mesh到这个东东上
      (bind _returnvalue (`AddComponent|NODE_AddSkeletalMeshComponent-0`))
      (`SkinnedMeshComponent.SetSkinnedAssetAndUpdate` _returnvalue (`self.WeaponMesh`) true)
      (bind _sucess_ (`/Game/TopDownBP/Blueprints/TopDownCharacter.EquipWeapon` _astop_down_character self))
      (return _sucess_))
    (:`CastFailed`
      (return false))))

(fn `UserConstructionScript`
  (`parent.UserConstructionScript`))
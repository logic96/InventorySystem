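; Item_ManaPotion is an inventory item that restores a fixed amount of mana to the player's character when used.
; OnUse casts the inventory's owning character to TopDownCharacter, then calls IncreaseMana and returns true if current MP is below the maximum.
; If MP is full or the cast fails it returns false, but the item actor destroys itself on every path.
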(fn `OnUse`
  (returns (`Sucess?` :type Boolean))
  (bind _astop_down_character (cast `/Game/TopDownBP/Blueprints/TopDownCharacter` (`/Game/InventorySystem/Blueprints/BP_Inventory.CharacterRef` (`self.InventoryRef`)))
    (:`then`
      (if (< (`/Game/TopDownBP/Blueprints/TopDownCharacter.CurrentMP` _astop_down_character) (`/Game/TopDownBP/Blueprints/TopDownCharacter.MaxMP` _astop_down_character))
        (`/Game/TopDownBP/Blueprints/TopDownCharacter.IncreaseMana` _astop_down_character 10)
        (`self.K2_DestroyActor`)
        (return true)
        (else
          (`self.K2_DestroyActor`)
          (return false))))
    (:`CastFailed`
      (`self.K2_DestroyActor`)
      (return false))))

(fn `UserConstructionScript`
  (`parent.UserConstructionScript`))
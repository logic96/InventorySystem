(event `self.OnUse`
  (`KismetSystemLibrary.PrintString` (`KismetStringLibrary.Concat_StrStr` "你装备了" (`KismetTextLibrary.Conv_TextToString` (`.Name_2_74B1ACCF44C51B4B4A0B12A45DA0F025` (break `/Game/InventorySystem/Blueprints/S_ItemInfo` (`self.ItemInfo`)))))))

(fn `UserConstructionScript`
  (`parent.UserConstructionScript`))
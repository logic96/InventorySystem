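; Old map inventory item that opens a map screen when used.
; OnUse disables the inventory widget, shows the main widget's map widget, hands it a reference to this actor and switches input to UI-only.
; OnClose re-enables the inventory, hides the map, restores game-and-UI input, then destroys the item actor.
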(fn `OnClose`
  (`Widget.SetIsEnabled` (`/Game/InventorySystem/Widget/W_MainWidget.InventoryWidget` (`/Game/InventorySystem/Blueprints/BP_Inventory.MainWidgetRef` (`self.InventoryRef`))) true)
  (`Widget.SetVisibility` (`/Game/InventorySystem/Widget/W_MainWidget.W_Map` (`/Game/InventorySystem/Blueprints/BP_Inventory.MainWidgetRef` (`self.InventoryRef`))) "Hidden")
  (`WidgetBlueprintLibrary.SetInputMode_GameAndUIEx` (`GameplayStatics.GetPlayerController` 0) null "DoNotLock" false)
  (`self.K2_DestroyActor`))

(fn `OnUse`
  (returns (`Sucess?` :type Boolean))
  (bind _w_map (`/Game/InventorySystem/Widget/W_MainWidget.W_Map` (`/Game/InventorySystem/Blueprints/BP_Inventory.MainWidgetRef` (`self.InventoryRef`))))
  (`Widget.SetIsEnabled` (`/Game/InventorySystem/Widget/W_MainWidget.InventoryWidget` (`/Game/InventorySystem/Blueprints/BP_Inventory.MainWidgetRef` (`self.InventoryRef`))) false)
  (set `/Game/InventorySystem/Widget/W_Map.MapActorRef` self _w_map)
  (`Widget.SetVisibility` _w_map "Visible")
  (`WidgetBlueprintLibrary.SetInputMode_UIOnlyEx` (`GameplayStatics.GetPlayerController` 0) _w_map)
  (return true))

(fn `UserConstructionScript`)
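; Merchant actor that opens a shop for the top-down character in the inventory system.
; Its sphere overlap shows or hides the merchant text and sets or clears itself as the character's nearby merchant.
; OnInteract creates a centered shop widget linked to merchant and character, hides the inventory, flags the shop open and stops movement.
; OnShopClosed removes the widget, clears the flag and restores walking.
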(event `self.Sphere.OnComponentBeginOverlap`
  (params (OverlappedComponent :type "PrimitiveComponent Object Reference") (OtherActor :type "Actor Object Reference") (OtherComp :type "PrimitiveComponent Object Reference") (OtherBodyIndex :type Integer) (bFromSweep :type Boolean) (SweepResult :type "HitResult Structure (by ref)"))
  (bind _astop_down_character (cast `/Game/TopDownBP/Blueprints/TopDownCharacter` OtherActor))
  (`SceneComponent.SetVisibility` (`self.MerchantText`) true false)
  (set `/Game/TopDownBP/Blueprints/TopDownCharacter.NearbyMerchant` self _astop_down_character))

(event `self.Sphere.OnComponentEndOverlap`
  (params (OverlappedComponent :type "PrimitiveComponent Object Reference") (OtherActor :type "Actor Object Reference") (OtherComp :type "PrimitiveComponent Object Reference") (OtherBodyIndex :type Integer))
  (bind _astop_down_character (cast `/Game/TopDownBP/Blueprints/TopDownCharacter` OtherActor))
  (`SceneComponent.SetVisibility` (`self.MerchantText`) false false)
  (set `/Game/TopDownBP/Blueprints/TopDownCharacter.NearbyMerchant` null _astop_down_character))

(fn `OnInteract`
  (params (CharacterRef :type "Character Object Reference"))
  (bind _shopwidget (`self.ShopWidget`))
  (bind _output_get (set `self.CharacterRef` CharacterRef))
  (bind _astop_down_character (cast `/Game/TopDownBP/Blueprints/TopDownCharacter` _output_get))
  (bind _returnvalue (`|CreateWidget` "/Game/InventorySystem/Widget/W_ShopWidget.W_ShopWidget_C" null self (`self.CharacterRef`)))
  (set `self.ShopWidget` _returnvalue)
  (`UserWidget.SetPositionInViewport` _shopwidget (0.0 0.0) false)
  (`UserWidget.SetAnchorsInViewport` _shopwidget (make `Anchors` (0.5 0.5) (0.5 0.5)))
  (`UserWidget.SetAlignmentInViewport` _shopwidget (0.5 0.5))
  (`UserWidget.AddToViewport` _shopwidget 5)
  (`/Game/InventorySystem/Blueprints/BP_Inventory.HideInventory` (`/Game/TopDownBP/Blueprints/TopDownCharacter.InventoryRef` _astop_down_character))
  (set `/Game/TopDownBP/Blueprints/TopDownCharacter.IsShopOpen` true _astop_down_character)
  (bind _charactermovement (`Character.CharacterMovement` _astop_down_character))
  (`CharacterMovementComponent.DisableMovement` _charactermovement)
  (`MovementComponent.StopMovementImmediately` _charactermovement))

(fn `OnShopClosed`
  (bind _astop_down_character (cast `/Game/TopDownBP/Blueprints/TopDownCharacter` (`self.CharacterRef`)))
  (set `/Game/TopDownBP/Blueprints/TopDownCharacter.IsShopOpen` false _astop_down_character)
  (`CharacterMovementComponent.SetMovementMode` (`Character.CharacterMovement` _astop_down_character) "MOVE_Walking" 0)
  (`Widget.RemoveFromParent` (`self.ShopWidget`)))

(fn `UserConstructionScript`)